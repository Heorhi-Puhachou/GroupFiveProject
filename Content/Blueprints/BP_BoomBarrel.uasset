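; BP_BoomBarrel is an explosive barrel actor that blows up when damaged or hit.
; Damage triggers the blast after a short delay, so nearby barrels can chain-react, while a hit detonates it immediately.
; A one-shot IsExploded guard runs the explosion: sound, scaled particle emitter, RadialForce impulse and radial damage around the barrel, then the actor destroys itself.
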(event EventBeginPlay)

(event Collision|EventActorBeginOverlap
  (params (OtherActor :type Actor%20Object%20Reference)))

(event EventTick
  (params (DeltaSeconds :type Float%20%28single-precision%29)))

(event Collision|EventHit
  (params (MyComp :type Primitive%20Component%20Object%20Reference) (Other :type Actor%20Object%20Reference) (OtherComp :type Primitive%20Component%20Object%20Reference) (bSelfMoved :type Boolean) (HitLocation :type Vector :default "0, 0, 0") (HitNormal :type Vector :default "0, 0, 0") (NormalImpulse :type Vector :default "0, 0, 0") (Hit :type Hit%20Result%20Structure%20%28by%20ref%29))
  (bind _returnvalue (Transformation|GetActorLocation))
  (if (not (Variables|Default|GetisExploded))
    (Variables|Default|SetisExploded true)
    (Audio|PlaySoundatLocation "/Game/StarterContent/Audio/Explosion01.Explosion01" _returnvalue "0, 0, 0" 1.0 1.0 0.0 0 0 0 0)
    (Effects|SpawnEmitteratLocation "/Game/StarterContent/Particles/P_Explosion.P_Explosion" _returnvalue "0, 0, 0" "2.000000,4.000000,2.000000")
    (Class|RadialForceComponent|FireImpulse (Variables|Default|GetRadialForce))
    (Game|Damage|ApplyRadialDamage 1e+02 _returnvalue 3e+02 0 0 self 0 false "ECC_Visibility")
    (Actor|DestroyActor)))

(event Game|Damage|EventAnyDamage
  (params (Damage :type Float%20%28single-precision%29) (DamageType :type Damage%20Type%20Object%20Reference) (InstigatedBy :type Controller%20Object%20Reference) (DamageCauser :type Actor%20Object%20Reference))
  (bind _returnvalue (Transformation|GetActorLocation))
  (Utilities|FlowControl|Delay 0.2)
  (if (not (Variables|Default|GetisExploded))
    (Variables|Default|SetisExploded true)
    (Audio|PlaySoundatLocation "/Game/StarterContent/Audio/Explosion01.Explosion01" _returnvalue "0, 0, 0" 1.0 1.0 0.0 0 0 0 0)
    (Effects|SpawnEmitteratLocation "/Game/StarterContent/Particles/P_Explosion.P_Explosion" _returnvalue "0, 0, 0" "2.000000,4.000000,2.000000")
    (Class|RadialForceComponent|FireImpulse (Variables|Default|GetRadialForce))
    (Game|Damage|ApplyRadialDamage 1e+02 _returnvalue 3e+02 0 0 self 0 false "ECC_Visibility")
    (Actor|DestroyActor)))

(fn ConstructionScript)